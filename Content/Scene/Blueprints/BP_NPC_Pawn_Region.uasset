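; Region actor that streams NPCs in and out as a BPI_Char actor enters or leaves its bounds.
; On entry, it spawns BT_AI-driven NPCs at each unused BP_NPC_Pawn point inside and links each NPC to its point.
; On exit, unless BackToStart is set, it destroys NPCs still inside and frees their points.
; A visibility trace from the player spares NPCs when it hits an NPC.
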(event Collision|EventActorBeginOverlap
  (params (OtherActor :type Actor%20Object%20Reference))
  (if (Utilities|DoesObjectImplementInterface OtherActor "/Game/FirstPersonBP/Interfaces/BPI_Char.BPI_Char_C")
    ;[1 1 1] 添加敌人
    (for _array_element (Collision|GetOverlappingActors "/Game/NPC/Blueprints/BP_NPC_Pawn.BP_NPC_Pawn_C" :!class /Script/Engine.Actor)
      (bind _asbp_npc_pawn (Utilities|Casting|CastToBP_NPC_Pawn _array_element))
      (if (not (Variables|/Game/NPC/Blueprints/BP_NPC_Pawn.BP_NPC_Pawn_C|GetbPawned _asbp_npc_pawn))
        (bind _returnvalue (AI|SpawnAIFromClass (Variables|/Game/NPC/Blueprints/BP_NPC_Pawn.BP_NPC_Pawn_C|GetNPCType _asbp_npc_pawn) "/Game/NPC/AI/Enemy/BT_AI.BT_AI" (Transformation|GetActorLocation _asbp_npc_pawn) "0, 0, 0" false))
        (bind _asbp_npc (Utilities|Casting|CastToBP_NPC _returnvalue))
        (bind _output_get (Variables|/Game/NPC/Blueprints/BP_NPC.BP_NPC_C|SetPawnPoint _asbp_npc _asbp_npc_pawn))
        (Variables|/Game/NPC/Blueprints/BP_NPC_Pawn.BP_NPC_Pawn_C|SetbPawned _output_get true)))))

(event Collision|EventActorEndOverlap
  (params (OtherActor :type Actor%20Object%20Reference))
  (bind _assim_game_instance (Utilities|Casting|CastToSIM_GameInstance (Game|GetGameInstance)))
  (if (not (Variables|/Game/GameSave/SIM_GameInstance.SIM_GameInstance_C|GetbBackToStart _assim_game_instance))
    (if (Utilities|DoesObjectImplementInterface OtherActor "/Game/FirstPersonBP/Interfaces/BPI_Char.BPI_Char_C")
      ;[1 1 1] 移除敌人
      (Utilities|Array|Clear (Variables|Default|GetDeleteList))
      (for _array_element (Collision|GetOverlappingActors "/Game/NPC/Blueprints/BP_NPC.BP_NPC_C" :!class /Script/Engine.Actor)
        (bind _bable (CallFunction|DeleteAble _array_element))
        (if _bable
          (Utilities|Array|Add (Variables|Default|GetDeleteList) _array_element)))
      (for _array_element_2 (Variables|Default|GetDeleteList)
        (bind _asbp_npc (Utilities|Casting|CastToBP_NPC _array_element_2))
        (Variables|/Game/NPC/Blueprints/BP_NPC_Pawn.BP_NPC_Pawn_C|SetbPawned (Variables|/Game/NPC/Blueprints/BP_NPC.BP_NPC_C|GetPawnPoint _asbp_npc) false)
        (Actor|DestroyActor _array_element_2)))))

(fn ConstructionScript)

(fn DeleteAble
  (params (DeleteActor :type Actor%20Object%20Reference))
  (bind (_outhit _returnvalue) (Collision|LineTraceByChannel (Transformation|GetActorLocation (Game|GetPlayerCharacter 0)) (Transformation|GetActorLocation DeleteActor) "TraceTypeQuery1" false 0 "None"))
  (return (Math|Boolean|ORBoolean (not _returnvalue) (not (Utilities|DoesObjectImplementInterface (.hitactor _outhit) "/Game/NPC/Interfaces/BPI_NPC.BPI_NPC_C")) false)))