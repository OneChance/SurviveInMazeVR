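; Base enemy AI character Blueprint that handles attacking a blackboard target and changing run speed.
; AttackEvent plays an animation, fires audio, effect hook and spark emitter at half the animation length, then applies damage through BPI_Char when it ends.
; AttackRangeOut triggers the attack animation cancel, and SpeedChange offsets RunSpeed from its base.
; AttackAnim, AttackAnimCancel_0 and AttackEffectTarget are empty functions here.
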(event Custom|AttackEvent
  (bind _returnvalue (Pawn|GetController))
  (bind _target (Variables|Default|GetTarget))
  (bind _animlength (Variables|Component|GetAnimLength))
  (bind _returnvalue_2 (AI|GetBlackboard _returnvalue))
  (bind _returnvalue_3 (* _animlength 0.5))
  (bind _returnvalue_4 (AI|Components|Blackboard|GetValueasObject _returnvalue_2 _target))
  ;[1 1 1] 攻击
  (bind _asbpi_char (Utilities|Casting|CastToBPI_Char _returnvalue_4))
  (CallFunction|AttackAnim)
  (Utilities|FlowControl|Delay _returnvalue_3)
  (Audio|Components|Audio|Play (Variables|Default|GetAttackAudio) 0.0)
  (CallFunction|AttackEffectTarget)
  (Audio|PlaySound2D "/Game/Audio/NPC/Enemy/attack_on.attack_on" 0.3)
  (bind _asactor (Utilities|Casting|CastToActor _returnvalue_4))
  (Effects|SpawnEmitteratLocation "/Game/Effects/ParticleSystems/P_spark_burst2.P_spark_burst2" (+ (Transformation|GetActorLocation _asactor) (* (Transformation|GetActorForwardVector _asactor) 80) (* (Transformation|GetActorUpVector _asactor) 45)))
  (Utilities|FlowControl|Delay _returnvalue_3)
  (Default|HealthChange _asbpi_char (Variables|Settings|GetDamage)))

(event Custom|AttackRangeOut
  ;[1 1 1] 取消攻击
  (CallFunction|NotiAttackAnimCancel))

(event Custom|SpeedChange
  (params (SpeedAdd :type Float%20%28single-precision%29))
  ;[1 1 1] 速度变化
  (Variables|Settings|SetRunSpeed (+ (Variables|Settings|GetRunSpeedBase) SpeedAdd)))

(fn ConstructionScript
  (|CallParentFunction))

(fn AttackAnim)

(fn AttackAnimCancel0)

(fn AttackEffectTarget)