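; Goblin enemy NPC Blueprint that supplies attack animation, weapon attachment and death reporting on top of its parent class.
; AttackAnim uses a cached reference to the goblin's Mixamo Anim Blueprint to raise its EnableAttack flag, and NotiAttackAnimCancel clears that flag.
; The construction script snaps the weapon to the mesh's Weapon socket after running the parent's.
; Killed notifies the game mode through NPCKilledMessage.
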(event EventAttackAnim
  ;[1 1 1] Attack
  (if (== (Variables|Default|GetAnim) 0)
    (bind _asmixamo_anim_bp_goblin (Utilities|Casting|CastToMixamoAnimBP_Goblin (Components|SkeletalMesh|GetAnimInstance (Variables|Character|GetMesh))))
    (Variables|Default|SetAnim _asmixamo_anim_bp_goblin))
  (if (not (Variables|/Game/MixamoAnimPack/Mixamo_Goblin/Anims/MixamoAnimBP_Goblin.MixamoAnimBP_Goblin_C|GetEnableAttack (Variables|Default|GetAnim)))
    (Variables|/Game/MixamoAnimPack/Mixamo_Goblin/Anims/MixamoAnimBP_Goblin.MixamoAnimBP_Goblin_C|SetEnableAttack (Variables|Default|GetAnim) true)))

(event EventNotiAttackAnimCancel
  ;[1 1 1] 停止攻击
  (bind _asmixamo_anim_bp_goblin (Utilities|Casting|CastToMixamoAnimBP_Goblin (Components|SkeletalMesh|GetAnimInstance (Variables|Character|GetMesh))))
  (Variables|/Game/MixamoAnimPack/Mixamo_Goblin/Anims/MixamoAnimBP_Goblin.MixamoAnimBP_Goblin_C|SetEnableAttack _asmixamo_anim_bp_goblin false))

(event EventKilled
  (Class|BPIGameMode|NPCKilled(Message) (Game|GetGameMode) 1))

(fn ConstructionScript
  (|CallParentFunction)
  (Class|SceneComponent|Attachto (Variables|Default|GetWeapon) (Variables|Character|GetMesh) "Weapon" "SnapToTargetIncludingScale" true))