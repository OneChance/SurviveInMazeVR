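; Vampire enemy NPC that drives its attack animation, spawns an attack effect and reports its death to the game mode.
; Attack events toggle EnableAttack on the Mixamo vampire AnimBP, caching the instance when enabling.
; The attack spawns a timed electricity emitter at an offset from the current target, also cleaned up if the vampire is destroyed mid-effect.
; The construction script snaps the weapon to the mesh's Weapon socket.
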(event Custom|对象销毁
  (params (DestroyedActor :type Actor%20Object%20Reference))
  ;[1 1 1] 绑定销毁事件，如果当前有正在播放的特效，一起销毁
  (if (Variables|Default|GetbEffect)
    (Components|DestroyComponent (Variables|Default|GetCurrentEffect))))

(event EventAttackAnim
  ;[1 1 1] 攻击动画
  (if (== (Variables|Default|GetAnim) 0)
    (bind _asmixamo_anim_bp_vampire (Utilities|Casting|CastToMixamoAnimBP_Vampire (Components|SkeletalMesh|GetAnimInstance (Variables|Character|GetMesh))))
    (Variables|Default|SetAnim _asmixamo_anim_bp_vampire))
  (if (not (Variables|/Game/MixamoAnimPack/Mixamo_Vampire/Anims/MixamoAnimBP_Vampire.MixamoAnimBP_Vampire_C|GetEnableAttack (Variables|Default|GetAnim)))
    (Variables|/Game/MixamoAnimPack/Mixamo_Vampire/Anims/MixamoAnimBP_Vampire.MixamoAnimBP_Vampire_C|SetEnableAttack (Variables|Default|GetAnim) true)))

(event EventAttackEffectTarget
  (bind _currenttarget (Variables|Default|GetCurrentTarget))
  ;[1 1 1] 攻击特效
  (bind _returnvalue (Effects|SpawnEmitteratLocation "/Game/Effects/ParticleSystems/P_electricity_DEMOFNL.P_electricity_DEMOFNL" (+ (+ (Transformation|GetActorLocation _currenttarget) (* (Transformation|GetActorUpVector _currenttarget) -8e+01)) (* (Transformation|GetActorForwardVector _currenttarget) 1.5e+02)) "90.000000,0,0.0"))
  (Variables|Default|SetCurrentEffect _returnvalue)
  (Variables|Default|SetbEffect true)
  (Utilities|FlowControl|Delay 1.0)
  (Components|DestroyComponent (Variables|Default|GetCurrentEffect))
  (Variables|Default|SetbEffect false))

(event EventBeginPlay
  ;[1 1 1] 绑定销毁事件，如果当前有正在播放的特效，一起销毁
  (EventDispatchers|BindEventtoOnDestroyed (delegate Custom|对象销毁)))

(event EventKilled
  (Class|BPIGameMode|NPCKilled(Message) (Game|GetGameMode) 3))

(event EventNotiAttackAnimCancel
  ;[1 1 1] 取消攻击
  (bind _asmixamo_anim_bp_vampire (Utilities|Casting|CastToMixamoAnimBP_Vampire (Components|SkeletalMesh|GetAnimInstance (Variables|Character|GetMesh))))
  (Variables|/Game/MixamoAnimPack/Mixamo_Vampire/Anims/MixamoAnimBP_Vampire.MixamoAnimBP_Vampire_C|SetEnableAttack _asmixamo_anim_bp_vampire false))

(fn ConstructionScript
  (|CallParentFunction)
  (Class|SceneComponent|Attachto (Variables|Default|GetWeapon) (Variables|Character|GetMesh) "Weapon" "SnapToTargetIncludingScale" true))