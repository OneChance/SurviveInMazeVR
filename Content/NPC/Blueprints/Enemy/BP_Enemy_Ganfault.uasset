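; Ganfault enemy NPC Blueprint that drives its attack animation and reports its death to the game mode.
; The attack event caches the Mixamo anim instance on first use and raises its EnableAttack flag, which the cancel notification clears.
; On death it sends the NPC killed message with its own ID.
; The construction script runs the parent's, then snaps the weapon to the mesh's Weapon socket.
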(event EventAttackAnim
  ;[1 1 1] 攻击动画
  (if (== (Variables|Default|GetAnim) 0)
    (bind _asmixamo_anim_bp_gan_faul (Utilities|Casting|CastToMixamoAnimBP_GanFaul (Components|SkeletalMesh|GetAnimInstance (Variables|Character|GetMesh))))
    (Variables|Default|SetAnim _asmixamo_anim_bp_gan_faul))
  (if (not (Variables|/Game/MixamoAnimPack/Mixamo_Ganfault/Anims/MixamoAnimBP_GanFaul.MixamoAnimBP_GanFaul_C|GetEnableAttack (Variables|Default|GetAnim)))
    (Variables|/Game/MixamoAnimPack/Mixamo_Ganfault/Anims/MixamoAnimBP_GanFaul.MixamoAnimBP_GanFaul_C|SetEnableAttack (Variables|Default|GetAnim) true)))

(event EventNotiAttackAnimCancel
  ;[1 1 1] 取消攻击
  (bind _asmixamo_anim_bp_gan_faul (Utilities|Casting|CastToMixamoAnimBP_GanFaul (Components|SkeletalMesh|GetAnimInstance (Variables|Character|GetMesh))))
  (Variables|/Game/MixamoAnimPack/Mixamo_Ganfault/Anims/MixamoAnimBP_GanFaul.MixamoAnimBP_GanFaul_C|SetEnableAttack _asmixamo_anim_bp_gan_faul false))

(event EventKilled
  (Class|BPIGameMode|NPCKilled(Message) (Game|GetGameMode) 5))

(fn ConstructionScript
  (|CallParentFunction)
  (Class|SceneComponent|Attachto (Variables|Default|GetWeapon) (Variables|Character|GetMesh) "Weapon" "SnapToTargetIncludingScale" true))