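; Base NPC character with health, target threat tracking, alert icon and speed-pitched footsteps, with empty hooks for death and attack cancel.
; Attackers become priority targets; Tick clears dead targets, or ones whose line-of-sight loss exceeds a timer, from the AI Blackboard.
; The Blackboard target also drives the alert and footstep pitch, while the patrol threat timer is unwired.
; Death plays explosion effects and spawns a random, level-scaled pickup chosen at construction.
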(event EventTick
  (params (DeltaSeconds :type Float%20%28single-precision%29))
  (Utilities|FlowControl|Sequence
    (:then_0
      ;[1 1 1] 目标仇恨移除计时
      (|TargetRemoveByTimer DeltaSeconds))
    (:then_1
      ;[1 1 1] 脚步声
      (|StepSound))
    (:then_2
      ;[1 1 1] 发现目标
      (|FindTargetAlert))))

(event EventHealthChange
  (params (ChangeValue :type Integer))
  (bind _self self)
  (bind _self_2 self)
  (bind _returnvalue (Transformation|GetActorLocation _self))
  ;[1 1 1] 生命值变化
  (bind _output_get (Variables|Settings|SetCurrentHealth (Math|Integer|Max(Integer) (Math|Integer|Min(Integer) (+ (Variables|Settings|GetCurrentHealth) ChangeValue) (Variables|Settings|GetMaxHealth)))))
  (if (== _output_get 0)
    (Effects|SpawnEmitteratLocation "/Game/Effects/ParticleSystems/P_Explosion_Bomb.P_Explosion_Bomb" _returnvalue)
    (Audio|PlaySoundatLocation "/Game/Audio/NPC/Enemy/explosion.explosion" _returnvalue "0, 0, 0" 0.4)
    (Audio|PlaySoundatLocation (Variables|/Script/Engine.AudioComponent|GetSound (Variables|Default|GetDeadAudio)) _returnvalue "0, 0, 0" 0.4)
    (for _array_element (Variables|Default|GetPickups _self_2)
      (bind _returnvalue_2 (Game|SpawnActorfromClass (.pclass _array_element) (Math|Transform|MakeTransform (+ (Transformation|GetActorLocation _self_2) "0, 0,-50.000000") "0, 0, 0" "1,1,1") "Undefined" 0 0))
      (Variables|/Game/Pickups/Blueprints/Pickups.Pickups_C|SetPNum _returnvalue_2 (.pnum _array_element)))
    (CallFunction|Killed)
    (Actor|DestroyActor)))

(event EventAttacked
  (params (AttackedBy :type Actor%20Object%20Reference))
  ;[1 1 1] 当被攻击时 直接锁定目标
  (Variables|Default|SetTargetWhoAttackActor AttackedBy)
  (Variables|Default|SetAttackedThreatRemoveTimer 0.0))

(fn ConstructionScript
  (CallFunction|SetPickupsbyLevel (Variables|Settings|GetLevel)))

(fn TargetIsVisble
  (params (Target :type Actor%20Object%20Reference))
  (bind _returnvalue (Collision|LineTraceByChannel (Transformation|GetActorLocation) (Transformation|GetActorLocation Target) "TraceTypeQuery1" false 0 "None"))
  (return (not _returnvalue)))

(fn SetPickupsbyLevel
  (params (Level :type Integer))
  (bind _returnvalue (Math|Random|RandomIntegerinRange 1 3))
  (bind _returnvalue_2 (* _returnvalue Level))
  (switch int (Math|Random|RandomIntegerinRange 0 2)
    (:0
      (Utilities|Array|Add (Variables|Default|GetPickups) (Utilities|Struct|MakePickupInfo "" _returnvalue_2 "/Game/Pickups/Blueprints/Pickups_Ammo.Pickups_Ammo_C")))
    (:1
      (Utilities|Array|Add (Variables|Default|GetPickups) (Utilities|Struct|MakePickupInfo "" _returnvalue_2 "/Game/Pickups/Blueprints/Pickups_Battery.Pickups_Battery_C")))
    (:2
      (Utilities|Array|Add (Variables|Default|GetPickups) (Utilities|Struct|MakePickupInfo "" _returnvalue_2 "/Game/Pickups/Blueprints/Pickups_Battery_Light.Pickups_Battery_Light_C")))))

(fn IsAlive
  (params (Target :type Actor%20Object%20Reference))
  (bind _asfirst_person_character (Utilities|Casting|CastToFirstPersonCharacter Target))
  (return (> (Variables|/Game/FirstPersonBP/Blueprints/FirstPersonCharacter.FirstPersonCharacter_C|GetCurrentHealth _asfirst_person_character) 0)))

(fn NotiAttackAnimCancel)

(fn Killed)