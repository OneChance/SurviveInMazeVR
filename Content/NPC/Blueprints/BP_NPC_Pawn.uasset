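; BP_NPC_Pawn is an NPC pawn whose Billboard sprite reflects the enemy class set in NPCType.
; The construction script compares NPCType against the Ganfault, Goblin, Heraklios, Vampire and Vanguard enemy Blueprints through a chain of branches.
; A match assigns that enemy's sprite to the Billboard, and any other type leaves the sprite untouched.
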(fn ConstructionScript
  (if (== (Variables|Default|GetNPCType) "/Game/NPC/Blueprints/Enemy/BP_Enemy_Ganfault.BP_Enemy_Ganfault_C")
    (Rendering|Components|Sprite|SetSprite (Variables|Default|GetBillboard) "/Game/NPC/Blueprints/ganfault.ganfault")
    (elif (== (Variables|Default|GetNPCType) "/Game/NPC/Blueprints/Enemy/BP_Enemy_Goblin.BP_Enemy_Goblin_C")
      (Rendering|Components|Sprite|SetSprite (Variables|Default|GetBillboard) "/Game/NPC/Blueprints/goblin.goblin")
      (elif (== (Variables|Default|GetNPCType) "/Game/NPC/Blueprints/Enemy/BP_Enemy_Heraklios.BP_Enemy_Heraklios_C")
        (Rendering|Components|Sprite|SetSprite (Variables|Default|GetBillboard) "/Game/NPC/Blueprints/heraklios.heraklios")
        (elif (== (Variables|Default|GetNPCType) "/Game/NPC/Blueprints/Enemy/BP_Enemy_Vampire.BP_Enemy_Vampire_C")
          (Rendering|Components|Sprite|SetSprite (Variables|Default|GetBillboard) "/Game/NPC/Blueprints/v.v")
          (elif (== (Variables|Default|GetNPCType) "/Game/NPC/Blueprints/Enemy/BP_Enemy_vanguard.BP_Enemy_vanguard_C")
            (Rendering|Components|Sprite|SetSprite (Variables|Default|GetBillboard) "/Game/NPC/Blueprints/vanguard.vanguard")))))))