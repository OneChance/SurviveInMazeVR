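; Sky sphere Blueprint that renders sun, sky colors, clouds and stars through a dynamic material instance.
; The construction script derives sun direction, color and height from an optional directional light or SunHeight, then sets sky colors from height-driven curves or manual properties.
; UpdateSunDirection reapplies the light-driven values and curve colors, with a slightly different horizon falloff range.
; A CloudsTimeline drives cloud noise and speed, but nothing triggers it.
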(fn ConstructionScript
  (bind _returnvalue (Rendering|Material|CreateDynamicMaterialInstance (Variables|BP_SkySphere|GetSky%20Sphere%20mesh) 0 "/Game/SkySphere/M_Sky_Pan_Clds2_Inst.M_Sky_Pan_Clds2_Inst" :!class /Script/Engine.PrimitiveComponent))
  (Variables|Default|SetmySky%20Material _returnvalue)
  (if (Variables|Default|GetRefresh%20Material%20) ; Updating bool in details panel causes construction script to run again
    _
    (else
      _))
  (Variables|Default|SetRefresh%20Material%20 false)
  (Utilities|IsValid (Variables|Default|GetDirectional%20light%20actor) ; Has a directional light been assigned?
    (:Is%20Valid
      (Rendering|Material|SetVectorParameterValue (Variables|Default|GetmySky%20Material) "Light direction" (Math|Conversions|ToLinearColor(Vector) (Math|Rotator|GetRotationXVector (Transformation|GetActorRotation (Variables|Default|GetDirectional%20light%20actor)))) :!class /Script/Engine.MaterialInstanceDynamic)
      (Rendering|Material|SetVectorParameterValue (Variables|Default|GetmySky%20Material) "Sun color" (Math|Conversions|ToLinearColor(Color) (Variables|/Script/Engine.LightComponentBase|GetLightColor (Variables|/Script/Engine.Light|GetLightComponent (Variables|Default|GetDirectional%20light%20actor)))) :!class /Script/Engine.MaterialInstanceDynamic)
      (Variables|OverrideSettings|SetSun%20height (Math|Float|MapRangeUnclamped (.Pitch (Math|Rotator|BreakRotator (Transformation|GetActorRotation (Variables|Default|GetDirectional%20light%20actor)))) 0.0 -9e+01 0.0 1.0)))
    (:Is%20Not%20Valid
      (Rendering|Material|SetVectorParameterValue (Variables|Default|GetmySky%20Material) "Light direction" (Math|Conversions|ToLinearColor(Vector) (Math|Rotator|GetRotationXVector (Math|Rotator|MakeRotator 0.0 (Math|Float|MapRangeUnclamped (Variables|OverrideSettings|GetSun%20height) -1.0 1.0 9e+01 -9e+01) (.Yaw (Math|Rotator|BreakRotator (Transformation|GetActorRotation)))))) :!class /Script/Engine.MaterialInstanceDynamic)
      (Rendering|Material|SetVectorParameterValue (Variables|Default|GetmySky%20Material) "Sun color" (Math|Color|Lerp(LinearColor) "(R=1.000000,G=0.221000,B=0.040000,A=1.000000)" "(R=0.954000,G=0.901000,B=0.744120,A=1.000000)" (Math|Float|Clamp(Float) (+ (Variables|OverrideSettings|GetSun%20height) 0.2))) :!class /Script/Engine.MaterialInstanceDynamic)))
  (if (Variables|Default|GetColors%20determined%20by%20sun%20position)
    (Rendering|Material|SetVectorParameterValue (Variables|Default|GetmySky%20Material) "Horizon color" (Math|Curves|GetLinearColorValue (Variables|Default|GetHorizon%20color%20curve) (Variables|OverrideSettings|GetSun%20height)) :!class /Script/Engine.MaterialInstanceDynamic)
    (Rendering|Material|SetVectorParameterValue (Variables|Default|GetmySky%20Material) "Zenith color" (Math|Curves|GetLinearColorValue (Variables|Default|GetZenith%20color%20curve) (Variables|OverrideSettings|GetSun%20height)) :!class /Script/Engine.MaterialInstanceDynamic)
    (Rendering|Material|SetVectorParameterValue (Variables|Default|GetmySky%20Material) "Cloud color" (Math|Curves|GetLinearColorValue (Variables|Default|GetCloud%20color%20curve) (Variables|OverrideSettings|GetSun%20height)) :!class /Script/Engine.MaterialInstanceDynamic)
    (Rendering|Material|SetScalarParameterValue (Variables|Default|GetmySky%20Material) "Horizon falloff" (Math|Float|Lerp 3.0 7.0 (Math|Float|Absolute(Float) (Variables|OverrideSettings|GetSun%20height))) :!class /Script/Engine.MaterialInstanceDynamic)
    (else
      (Rendering|Material|SetVectorParameterValue (Variables|Default|GetmySky%20Material) "Horizon color" (Variables|OverrideSettings|GetHorizon%20color) :!class /Script/Engine.MaterialInstanceDynamic)
      (Rendering|Material|SetVectorParameterValue (Variables|Default|GetmySky%20Material) "Zenith color" (Variables|OverrideSettings|GetZenith%20Color) :!class /Script/Engine.MaterialInstanceDynamic)
      (Rendering|Material|SetVectorParameterValue (Variables|Default|GetmySky%20Material) "Overall color" (Variables|OverrideSettings|GetOverall%20Color) :!class /Script/Engine.MaterialInstanceDynamic)
      (Rendering|Material|SetVectorParameterValue (Variables|Default|GetmySky%20Material) "Cloud color" (Variables|OverrideSettings|GetCloud%20color) :!class /Script/Engine.MaterialInstanceDynamic)
      (Rendering|Material|SetScalarParameterValue (Variables|Default|GetmySky%20Material) "Horizon falloff" (Variables|OverrideSettings|GetHorizon%20Falloff) :!class /Script/Engine.MaterialInstanceDynamic)))
  (Rendering|Material|SetScalarParameterValue (Variables|Default|GetmySky%20Material) "Cloud speed" (Variables|Default|GetCloud%20speed) :!class /Script/Engine.MaterialInstanceDynamic)
  (Rendering|Material|SetScalarParameterValue (Variables|Default|GetmySky%20Material) "Sun brightness" (Variables|Default|GetSun%20brightness) :!class /Script/Engine.MaterialInstanceDynamic)
  (Rendering|Material|SetScalarParameterValue (Variables|Default|GetmySky%20Material) "Sun height" (Math|Float|SelectFloat (Math|Float|Absolute(Float) (Variables|OverrideSettings|GetSun%20height)) 0.0 (< (Variables|OverrideSettings|GetSun%20height) 0.0)) :!class /Script/Engine.MaterialInstanceDynamic)
  (Rendering|Material|SetScalarParameterValue (Variables|Default|GetmySky%20Material) "Cloud opacity" (Variables|Default|GetCloud%20opacity) :!class /Script/Engine.MaterialInstanceDynamic)
  (Rendering|Material|SetScalarParameterValue (Variables|Default|GetmySky%20Material) "Stars brightness" (Variables|Default|GetStars%20brightness) :!class /Script/Engine.MaterialInstanceDynamic))

(fn UpdateSunDirection
  (bind _mysky_material (Variables|Default|GetmySky%20Material))
  (bind _mysky_material_2 (Variables|Default|GetmySky%20Material))
  (Rendering|Material|SetVectorParameterValue _mysky_material_2 "Light direction" (Math|Conversions|ToLinearColor(Vector) (Math|Rotator|GetRotationXVector (Transformation|GetActorRotation (Variables|Default|GetDirectional%20light%20actor)))) :!class /Script/Engine.MaterialInstanceDynamic)
  (Rendering|Material|SetVectorParameterValue _mysky_material_2 "Sun color" (Math|Conversions|ToLinearColor(Color) (Variables|/Script/Engine.LightComponentBase|GetLightColor (Variables|/Script/Engine.Light|GetLightComponent (Variables|Default|GetDirectional%20light%20actor)))) :!class /Script/Engine.MaterialInstanceDynamic)
  (Variables|OverrideSettings|SetSun%20height (Math|Float|MapRangeUnclamped (.Pitch (Math|Rotator|BreakRotator (Transformation|GetActorRotation (Variables|Default|GetDirectional%20light%20actor)))) 0.0 -9e+01 0.0 1.0))
  (Rendering|Material|SetVectorParameterValue _mysky_material "Horizon color" (Math|Curves|GetLinearColorValue (Variables|Default|GetHorizon%20color%20curve) (Variables|OverrideSettings|GetSun%20height)) :!class /Script/Engine.MaterialInstanceDynamic)
  (Rendering|Material|SetVectorParameterValue _mysky_material "Zenith color" (Math|Curves|GetLinearColorValue (Variables|Default|GetZenith%20color%20curve) (Variables|OverrideSettings|GetSun%20height)) :!class /Script/Engine.MaterialInstanceDynamic)
  (Rendering|Material|SetVectorParameterValue _mysky_material "Cloud color" (Math|Curves|GetLinearColorValue (Variables|Default|GetCloud%20color%20curve) (Variables|OverrideSettings|GetSun%20height)) :!class /Script/Engine.MaterialInstanceDynamic)
  (Rendering|Material|SetScalarParameterValue _mysky_material "Horizon falloff" (Math|Float|Lerp 3.0 8.0 (Math|Float|Absolute(Float) (Variables|OverrideSettings|GetSun%20height))) :!class /Script/Engine.MaterialInstanceDynamic)
  (Rendering|Material|SetScalarParameterValue _mysky_material "Sun height" (Math|Float|SelectFloat (Math|Float|Absolute(Float) (Variables|OverrideSettings|GetSun%20height)) 0.0 (< (Variables|OverrideSettings|GetSun%20height) 0.0)) :!class /Script/Engine.MaterialInstanceDynamic))